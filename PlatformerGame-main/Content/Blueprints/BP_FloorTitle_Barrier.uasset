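; Floor barrier obstacle that kills BP_MainCharacter when the character hits its Wall3 component.
; Its construction script adds each instance to the RunGameMode BarriersArray.
; The WallsVisible event turns off Wall3 collision for a fixed delay, then restores it as query-only, ignoring its parameter and leaving visibility untouched.
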(event `self.Wall3.OnComponentHit`
  (params (HitComponent :type "PrimitiveComponent Object Reference") (OtherActor :type "Actor Object Reference") (OtherComp :type "PrimitiveComponent Object Reference") (NormalImpulse :type "Vector Structure") (Hit :type "HitResult Structure (by ref)"))
  (bind _asbp_main_character (cast `/Game/Blueprints/BP_MainCharacter` OtherActor))
  (`/Game/Blueprints/BP_MainCharacter.Death` _asbp_main_character))

(event `WallsVisible`
  (params (NewParam :type "StaticMeshSimulationComponent Object Reference"))
  (`PrimitiveComponent.SetCollisionEnabled` (`self.Wall3`) "NoCollision")
  (`KismetSystemLibrary.Delay` 10.0)
  (`PrimitiveComponent.SetCollisionEnabled` (`self.Wall3`) "QueryOnly"))

(fn `UserConstructionScript`
  (bind _asrun_game_mode (cast `/Game/Blueprints/RunGameMode` (`GameplayStatics.GetGameMode`)))
  (bind _output_get (set `/Game/Blueprints/RunGameMode.BarriersArray` (`/Game/Blueprints/RunGameMode.BarriersArray` _asrun_game_mode) _asrun_game_mode))
  (`KismetArrayLibrary.Array_Add` _output_get self))