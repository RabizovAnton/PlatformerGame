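; BP_Freezing_Bonus is a pickup that freezes the blockers in a run when the player character touches it.
; On mesh overlap with BP_MainCharacter, it plays the coin pickup sound at its location and destroys itself.
; It then loops over the RunGameMode's BlockersArray and calls Freeze on each BP_Blocker.
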(event `self.StaticMesh.OnComponentBeginOverlap`
  (params (OverlappedComponent :type "PrimitiveComponent Object Reference") (OtherActor :type "Actor Object Reference") (OtherComp :type "PrimitiveComponent Object Reference") (OtherBodyIndex :type Integer) (bFromSweep :type Boolean) (SweepResult :type "HitResult Structure (by ref)"))
  (cast `/Game/Blueprints/BP_MainCharacter` OtherActor)
  (`GameplayStatics.PlaySoundAtLocation` "/Game/StarterContent/Audio/CoinPickUpSound.CoinPickUpSound" (`self.K2_GetActorLocation`) (struct) 1.0 1.0 0.0 null null null)
  (`self.K2_DestroyActor`)
  (bind _asrun_game_mode (cast `/Game/Blueprints/RunGameMode` (`GameplayStatics.GetGameMode`)))
  (for _array_element (`/Game/Blueprints/RunGameMode.BlockersArray` _asrun_game_mode)
    (bind _asbp_blocker (cast `/Game/Blueprints/BP_Blocker` _array_element))
    (`/Game/Blueprints/BP_Blocker.Freeze` _asbp_blocker)))

(fn `UserConstructionScript`)