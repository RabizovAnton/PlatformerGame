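; BP_FloorTitle_Moveable is a movable floor tile Blueprint that travels between two relative locations.
; Its construction script sets the IsCornerOrMovable flag before calling the parent construction script.
; It then builds two InterpToMovement control points from Location1 and Location2 and applies the Duration variable to the movement.
; The event graph holds only disabled default events, so the movement component drives all motion.
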(fn `UserConstructionScript`
  (bind _interptomovement (`self.InterpToMovement`))
  (set `self.IsCornerOrMovable?` true)
  (`parent.UserConstructionScript`)
  (set `InterpToMovementComponent.ControlPoints` (`|MakeArray` (make `InterpControlPoint` (`self.Location1`)) (make `InterpControlPoint` (`self.Location2`))) _interptomovement)
  (set `InterpToMovementComponent.Duration` (`self.duration`) _interptomovement))