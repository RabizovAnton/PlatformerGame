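; Game mode for an endless-runner style level that builds the floor procedurally from random tiles.
; On BeginPlay it adds the Interface widget to the viewport and lays an initial run of tiles through AddFloorTitle.
; Each piece spawns at NextSpawnPoint, which then moves to that piece's attach transform to chain the track.
; A straight counter makes AddFloorTitle hand off to AddFloorCurve after several straights, which resets the count.
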(event `self.ReceiveBeginPlay`
  (bind _returnvalue (`|CreateWidget` "/Game/Blueprints/UMG/Interface.Interface_C"))
  (`UserWidget.AddToViewport` _returnvalue 0)
  (for _ (range 10)
    (`self.AddFloorTitle`)))

(fn `AddFloorCurve`
  (bind _floorcurves (`self.FloorCurves`))
  (bind _returnvalue (`|SpawnActorFromClass` (`|GetArrayItem` _floorcurves (`KismetMathLibrary.RandomIntegerInRange` 0 (`KismetArrayLibrary.Array_LastIndex` _floorcurves))) (`self.NextSpawnPoint`) "Undefined" "OverrideRootScale" null null))
  (bind _asbp_floor_title (cast `/Game/Blueprints/BP_FloorTitle` _returnvalue))
  (bind _attachtransform (`/Game/Blueprints/BP_FloorTitle.GetAttachTransform` _asbp_floor_title))
  (set `self.NextSpawnPoint` _attachtransform)
  (set `self.CurrentStraights` 0))

(fn `AddFloorTitle`
  (bind _floortitles (`self.FloorTitles`))
  (if (> (`self.CurrentStraights`) 5)
    (`self.AddFloorCurve`)
    (else
      (bind _returnvalue (`|SpawnActorFromClass` (`|GetArrayItem` _floortitles (`KismetMathLibrary.RandomIntegerInRange` 0 (`KismetArrayLibrary.Array_LastIndex` _floortitles))) (`self.NextSpawnPoint`) "Undefined" "OverrideRootScale" null null))
      (bind _asbp_floor_title (cast `/Game/Blueprints/BP_FloorTitle` _returnvalue))
      (bind _attachtransform (`/Game/Blueprints/BP_FloorTitle.GetAttachTransform` _asbp_floor_title))
      (set `self.NextSpawnPoint` _attachtransform)
      (set `self.CurrentStraights` (+ (`self.CurrentStraights`) 1)))))

(fn `UserConstructionScript`)