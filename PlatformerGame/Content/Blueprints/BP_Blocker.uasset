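; BP_Blocker is a moving obstacle that calls Death on BP_MainCharacter when its static mesh hits the player.
; Its construction script builds a two-point relative InterpToMovement path from Location1 and Location2, with a shorter duration on Level_3.
; The same script adds the blocker to the RunGameMode BlockersArray.
; A Freeze event halts movement by disabling the component's tick, then restores it after a ten-second delay.
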(event `self.StaticMesh.OnComponentHit`
  (params (HitComponent :type "PrimitiveComponent Object Reference") (OtherActor :type "Actor Object Reference") (OtherComp :type "PrimitiveComponent Object Reference") (NormalImpulse :type "Vector Structure") (Hit :type "HitResult Structure (by ref)"))
  (bind _asbp_main_character (cast `/Game/Blueprints/BP_MainCharacter` OtherActor))
  (`/Game/Blueprints/BP_MainCharacter.Death` _asbp_main_character))

(event `Freeze`
  (bind _interptomovement (`self.InterpToMovement`))
  (`ActorComponent.SetComponentTickEnabled` _interptomovement false)
  (`KismetSystemLibrary.Delay` 10.0)
  (`ActorComponent.SetComponentTickEnabled` _interptomovement true))

(fn `UserConstructionScript`
  (bind _interptomovement (`self.InterpToMovement`))
  (bind _returnvalue (`GameplayStatics.GetCurrentLevelName` true))
  (bind _returnvalue_2 (`GameplayStatics.GetCurrentLevelName` true))
  (bind _returnvalue_3 (`GameplayStatics.GetCurrentLevelName` true))
  (set `InterpToMovementComponent.ControlPoints` (`|MakeArray` (make `InterpControlPoint` (`self.Location1`)) (make `InterpControlPoint` (`self.Location2`))) _interptomovement)
  (if (`KismetStringLibrary.EqualEqual_StrStr` _returnvalue "Level_3")
    (set `InterpToMovementComponent.Duration` 0.5 _interptomovement)
    (bind _asrun_game_mode (cast `/Game/Blueprints/RunGameMode` (`GameplayStatics.GetGameMode`)))
    (`KismetArrayLibrary.Array_Add` (`/Game/Blueprints/RunGameMode.BlockersArray` _asrun_game_mode) self)
    (else
      (set `InterpToMovementComponent.Duration` 1.0 _interptomovement)
      (bind _asrun_game_mode_2 (cast `/Game/Blueprints/RunGameMode` (`GameplayStatics.GetGameMode`)))
      (`KismetArrayLibrary.Array_Add` (`/Game/Blueprints/RunGameMode.BlockersArray` _asrun_game_mode_2) self))))